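; BP_Plunger is a ball plunger that pulls back while charging and snaps forward on release.
; ChargePlunger plays a timeline that lerps PlungerMesh along local Y from rest to full pullback.
; StopCharge halts the timeline and uses MoveComponentTo to return the mesh to its origin almost instantly.
; GetBallSpawnLocation converts the relative BallLocation into world space through the actor transform.
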(event Custom|ChargePlunger
  ;[1 1 1] Charge Plunger
  ;;[1 1 1] Gradually move the plundger furthur back untill stopped into a location
  (bind _chargealpha (Timeline|ChargeTimeline PlayFromStart)
    (:Update
      ;;[1 1 1] Update the location of the plunger from 0.0 not charged to 150.0 fully charged
      (Transformation|SetRelativeLocation (Variables|Default|GetPlungerMesh) (Math|Vector|Lerp(Vector) "0, 0, 0" "0,150.000000, 0" _chargealpha) false false))))

(event Custom|StopCharge
  ;[1 1 1] stop charge
  ;;[1 1 1] Then 0 is to stop the charge.
  (Utilities|FlowControl|Sequence
    (:then_0
      ;[1 1 1] Charge Plunger
      ;;[1 1 1] Gradually move the plundger furthur back untill stopped into a location
      (bind _chargealpha (Timeline|ChargeTimeline Stop)
        (:Update
          ;;[1 1 1] Update the location of the plunger from 0.0 not charged to 150.0 fully charged
          (Transformation|SetRelativeLocation (Variables|Default|GetPlungerMesh) (Math|Vector|Lerp(Vector) "0, 0, 0" "0,150.000000, 0" _chargealpha) false false))))
    (:then_1
      ;;[1 1 1] Move a component to the intial postion 0.0 over a very short peroid of time of 0.1 seconds
      (Components|MoveComponentTo (Variables|Default|GetPlungerMesh) "0, 0, 0" "0, 0, 0" false false 0.1 false))))

(event EventBeginPlay)

(event Collision|EventActorBeginOverlap
  (params (OtherActor :type Actor%20Object%20Reference)))

(event EventTick
  (params (DeltaSeconds :type Float%20%28single-precision%29))
  ;[1 1 1] Charge Plunger
)

(fn ConstructionScript)

(fn GetBallSpawnLocation
  ;[1 1 1] Postition in the world where the ball should spawn at
  (return (Math|Transform|TransformLocation (Transformation|GetActorTransform) (Variables|Default|GetBallLocation))))