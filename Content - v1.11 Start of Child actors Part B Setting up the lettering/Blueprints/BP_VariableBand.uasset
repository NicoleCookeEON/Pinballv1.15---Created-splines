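; BP_VariableBand is a construction-script actor that builds two facing posts with a stretched band between them.
; It rotates Post1 toward the editable PostLocation, then adds a second post there with the same mesh, facing back.
; An extender mesh is added at Post1's transform, its X scale set from the distance between posts over 100, keeping Post1's Y and Z scale.
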(event EventBeginPlay)

(event Collision|EventActorBeginOverlap
  (params (OtherActor :type Actor%20Object%20Reference)))

(event EventTick
  (params (DeltaSeconds :type Float%20%28single-precision%29)))

(fn ConstructionScript
  (bind _postlocation (Variables|Default|GetPostLocation))
  (bind _post1 (Variables|Default|GetPost1))
  (bind _post1_2 (Variables|Default|GetPost1))
  (bind _returnvalue (Transformation|GetRelativeTransform _post1))
  (bind _scale (Math|Transform|BreakTransform _returnvalue))
  ;[1 1 1] This will rotate the static mesh
  (Transformation|SetRelativeRotation _post1_2 (Math|Rotator|FindLookatRotation (Variables|/Script/Engine.SceneComponent|GetRelativeLocation _post1_2) (Variables|Default|GetPostLocation)) false false)
  ;[1 1 1] Relative transform is going to be equal to the postLocation. Also the default rotation is going to be the oposite of FindLookAtRotation
  (bind _returnvalue_2 (AddComponent|AddStaticMeshComponent false (Math|Transform|MakeTransform _postlocation (Math|Rotator|FindLookatRotation _postlocation (Variables|/Script/Engine.SceneComponent|GetRelativeLocation (Variables|Default|GetPost1))))))
  ;[1 1 1] This creates the second post mesh that we move around
  (Components|StaticMesh|SetStaticMesh _returnvalue_2 (Variables|/Script/Engine.StaticMeshComponent|GetStaticMesh (Variables|Default|GetPost1)))
  ;[1 1 1] This is going to be the SM_BandExtender
  (bind _returnvalue_3 (AddComponent|AddStaticMeshComponent false _returnvalue))
  ;[1 1 1] Doing the math backwards on of the approx size. To connect the meshes together
  (Transformation|SetRelativeScale3D _returnvalue_3 (Math|Vector|MakeVector (/ (Math|Vector|VectorLength (- (Variables|/Script/Engine.SceneComponent|GetRelativeLocation (Variables|Default|GetPost1)) (Variables|Default|GetPostLocation))) 1e+02) (.y _scale) (.z _scale))))