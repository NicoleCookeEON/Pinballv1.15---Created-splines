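; Player controller for a pinball game that turns input into flipper, plunger and table tilt actions and creates the HUD.
; On BeginPlay it sorts flippers into left and right arrays by FlipType and caches the first plunger found.
; Input events flip or flop each side and charge or release the plunger.
; Tilt uses the game mode's limited TiltCount to impulse every ball sideways with a directional camera shake.
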(event Custom|DetectFlippers
  ;[1 1 1] Detect Flipper
  ;;[1 1 1] Go through the list and for every item that is in this list
  (bind _outactors (Actor|GetAllActorsOfClass "/Game/Blueprints/FLIPPER.Flipper_C"))
  ;;[1 1 1] Run the funciton off of Loop Body
  (for _array_element _outactors
    ;;[1 1 1] Look for if it is left flipper or a right flipper
    (switch Utilities|FlowControl|Switch|SwitchonFlipType (Variables|/Game/Blueprints/FLIPPER.Flipper_C|GetFlipType _array_element)
      (:NewEnumerator0
        ;;[1 1 1] If its a left flipper get the array and add to the array
        (Utilities|Array|Add (Variables|Default|GetLeftFlippers) _array_element))
      (:NewEnumerator1
        ;;[1 1 1] If its a right flipper get the array and add to the array
        (Utilities|Array|Add (Variables|Default|GetRightFlippers) _array_element)))))

(event Custom|CreatePlayerHUD
  ;[1 1 1] Create Player HUD
  (Viewport|RemoveAllWidgets)
  (bind _returnvalue (UserInterface|CreateWidget "/Game/Blueprints/PinballHUD.PinballHUD_C"))
  (UserInterface|Viewport|AddtoViewport _returnvalue 0))

(event Custom|DetectPlunger
  ;[1 1 1] Detect Plunger
  ;;[1 1 1] Go through the list and for every item that is in this list
  (bind _outactors (Actor|GetAllActorsOfClass "/Game/Blueprints/BP_Plunger.BP_Plunger_C"))
  ;;[1 1 1] Very first one that it finds is the plunger
  (Variables|Default|SetPlunger (Utilities|Array|Get(acopy) _outactors)))

(event EventBeginPlay
  ;[1 1 1] Begin Play
  (CallFunction|DetectFlippers)
  (CallFunction|DetectPlunger)
  (CallFunction|CreatePlayerHUD))

(event EventTick
  (params (DeltaSeconds :type Float%20%28single-precision%29)))

(event Input|ActionEvents|InputActionLeftFlipper
  (params (Key :type Key%20Structure :default "AnyKey"))
  (bind _leftflippers (Variables|Default|GetLeftFlippers))
  ;[1 1 1] Input left flipper
  (:Pressed
    (for _array_element _leftflippers
      ;;[1 1 1] We want every flipper to flip
      (Default|Flip _array_element)))
  (:Released
    (for _array_element_2 _leftflippers
      ;;[1 1 1] We want every flipper to flop
      (Default|Flop _array_element_2))))

(event Input|ActionEvents|InputActionRightFlipper
  (params (Key :type Key%20Structure :default "AnyKey"))
  (bind _rightflippers (Variables|Default|GetRightFlippers))
  ;[1 1 1] Input right flipper
  (:Pressed
    (for _array_element _rightflippers
      ;;[1 1 1] We want every flipper to flip
      (Default|Flip _array_element)))
  (:Released
    (for _array_element_2 _rightflippers
      ;;[1 1 1] We want every flipper to flop
      (Default|Flop _array_element_2))))

(event Input|ActionEvents|InputActionPlunger
  (params (Key :type Key%20Structure :default "AnyKey"))
  (bind _plunger (Variables|Default|GetPlunger))
  ;[1 1 1] Input plunger - functions are found in BP_Plunger
  (:Pressed
    (Default|ChargePlunger _plunger))
  (:Released
    (Default|StopCharge _plunger)))

(event Input|ActionEvents|InputActionLeftTilt
  (params (Key :type Key%20Structure :default "AnyKey"))
  ;[1 1 1] LeftTilt
  (:Pressed
    ;;[1 1 1] Tilt Function
    (CallFunction|Tilt "NewEnumerator0")))

(event Input|ActionEvents|InputActionRightTilt
  (params (Key :type Key%20Structure :default "AnyKey"))
  ;[1 1 1] RightTilt
  (:Pressed
    (CallFunction|Tilt "NewEnumerator1")))

(fn ConstructionScript)

(fn Tilt
  (params (TiltDirection :type FlipType%20Enum))
  (bind _returnvalue (Game|GetPlayerCameraManager 0))
  (bind _returnvalue_2 (Camera|GetCameraRotation _returnvalue))
  ;[1 1 1] Tilt direction - will select the direction we are going in
  (if (> (Variables|/Game/Blueprints/PinballGameMode.PinballGameMode_C|GetTiltCount (.AsPinball%20Game%20Mode (Utilities|Casting|CastToPinballGameMode (Game|GetGameMode)))) 0)
    (bind _outactors (Actor|GetAllActorsOfClass "/Game/Blueprints/Bp_Ball.Bp_Ball_C"))
    (if (>= (Utilities|Array|Length _outactors) 0)
      (for _array_element _outactors
        (Physics|AddImpulse (Variables|/Game/Blueprints/Bp_Ball.Bp_Ball_C|GetBall _array_element) (Utilities|Select :Index TiltDirection :NewEnumerator0 "500.000000,0,0" :NewEnumerator1 "-500.000000,0,0") "None" true)
        ;[1 1 1] Shakes the camera
        (Class|PlayerController|ClientPlayCameraShake "/Game/Blueprints/TiltShake.TiltShake_C" 1.0 "UserDefined" (Utilities|Select :Index TiltDirection :NewEnumerator0 _returnvalue_2 :NewEnumerator1 (Math|Rotator|CombineRotators _returnvalue_2 "0,180.000000, 0"))))
      ;[1 1 1] Remove a tilt
      (Math|Integer|DecrementInt (Variables|/Game/Blueprints/PinballGameMode.PinballGameMode_C|GetTiltCount (.AsPinball%20Game%20Mode (Utilities|Casting|CastToPinballGameMode (Game|GetGameMode))))))))