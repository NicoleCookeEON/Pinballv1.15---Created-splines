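; BP_ForceMovementZone is a zone that steers any overlapping Bp_Ball along the direction of its Arrow component.
; Each tick it converts the ball's velocity into arrow space and interpolates toward a target whose forward speed is clamped within a set range.
; AdoptionSpeed sets the blend rate, and the result returns to world space as the ball's physics linear velocity, replacing the current one.
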(event EventBeginPlay)

(event Collision|EventActorBeginOverlap
  (params (OtherActor :type Actor%20Object%20Reference)))

(event EventTick
  (params (DeltaSeconds :type Float%20%28single-precision%29))
  (for _array_element (Collision|GetOverlappingActors "/Game/Blueprints/Bp_Ball.Bp_Ball_C" :!class /Script/Engine.Actor)
    ;[1 1 1] Set the velocity on the ball
    (Physics|SetPhysicsLinearVelocity (Variables|/Game/Blueprints/Bp_Ball.Bp_Ball_C|GetBall (.AsBp%20Ball (Utilities|Casting|CastToBp_Ball _array_element))) (Math|Transform|TransformDirection (Transformation|GetWorldTransform (Variables|Default|GetArrow)) (Math|Interpolation|VInterpTo (Math|Transform|InverseTransformDirection (Transformation|GetWorldTransform (Variables|Default|GetArrow)) (Transformation|GetVelocity _array_element)) (Math|Vector|MakeVector (Math|Float|Clamp(Float) (.X (Math|Vector|BreakVector (Math|Transform|InverseTransformDirection (Transformation|GetWorldTransform (Variables|Default|GetArrow)) (Transformation|GetVelocity _array_element)))) 8e+02 1.9e+03) 0.0 0.0) (Utilities|Time|GetWorldDeltaSeconds) (Variables|Default|GetAdoptionSpeed))) false "None")))

(fn ConstructionScript)