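; BP_Slingshot is a pinball-style slingshot bumper that knocks the ball away when it overlaps.
; An overlapping Bp_Ball gets a strong impulse opposite the Capsule's forward vector, then the SlingBounce timeline plays.
; The timeline drives the PercentOut parameter on a dynamic M_MorphBand material, created in the construction script, to animate the static mesh's band through the material.
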(event EventBeginPlay)

(event Collision|EventActorBeginOverlap
  (params (OtherActor :type Actor%20Object%20Reference))
  ;[1 1 1] If the ball hits
  (bind _asbp_ball (Utilities|Casting|CastToBp_Ball OtherActor))
  (Physics|AddImpulse (Variables|/Game/Blueprints/Bp_Ball.Bp_Ball_C|GetBall _asbp_ball) (* (Math|Vector|GetForwardVector (Variables|Default|GetCapsule)) -2.5e+03) "None" false)
  ;[1 1 1] Not just one instance calculating one
  (bind _bounce (Timeline|SlingBounce Play)
    (:Update
      ;[1 1 1] This is in the construction script
      (bind _asmaterial_instance_dynamic (Utilities|Casting|CastToMaterialInstanceDynamic (Rendering|Material|GetMaterial (Variables|Default|GetStaticMesh) 2)))
      (Rendering|Material|SetScalarParameterValue _asmaterial_instance_dynamic "PercentOut" _bounce :!class /Script/Engine.MaterialInstanceDynamic))))

(event EventTick
  (params (DeltaSeconds :type Float%20%28single-precision%29)))

(fn ConstructionScript
  ;[1 1 1] Elemet index is in the material this is the second one (Yellow mat)
  (Rendering|Material|CreateDynamicMaterialInstance (Variables|Default|GetStaticMesh) 2 "/Game/Assets/M_MorphBand.M_MorphBand" :!class /Script/Engine.PrimitiveComponent))