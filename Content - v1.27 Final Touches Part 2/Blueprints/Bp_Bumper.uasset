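; Pinball bumper actor that knocks an overlapping Bp_Ball away and awards score through PinballGameMode.
; The overlap calls Bump, which applies a velocity-change impulse along the bumper-to-ball direction and plays an attached hit sound.
; The BumpLerp timeline then dips the mechanism and drives the point light intensity and emissive boost.
; The construction script creates the dynamic material instance used for that glow.
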(event Custom|Bump
  (params (Ball :type Bp%20Ball%20Object%20Reference))
  ;[1 1 1] When function is called - read in a refernce to the things we want to bump
  ;[1 1 1] Add impulse
  ;;[1 1 1] Read in a direction we want the ball to go in
  (Physics|AddImpulse (Variables|/Game/Blueprints/Bp_Ball.Bp_Ball_C|GetBall Ball) (* (Math|Vector|GetUnitDirection(Vector) (Transformation|GetActorLocation) (Transformation|GetActorLocation Ball)) 2.5e+03) "None" true)
  ;[1 1 1] Spawn sound attached
  ;;[1 1 1] Added before the timline else the sounds would be sounding every milly second instead of one time
  (Audio|SpawnSoundAttached "/Game/Assets/Sounds/BumperHit.BumperHit" (Variables|Default|GetBumperMesh))
  ;[1 1 1] Add score - Add current GameMode, cast GameMode to be a pinball game mode, add some score to it
  (bind _aspinball_game_mode (Utilities|Casting|CastToPinballGameMode (Game|GetGameMode))
    (:then
      (Default|AddScore _aspinball_game_mode 1e+01)
      ;[1 1 1] Bump lerp to make the animation
      ;;[1 1 1] Timeline - Creating a mini graph of time vs variable let it drive any aparmaters with in any blueprint. - Double click to see more
      (bind _bumpalpha (Timeline|BumpLerp PlayFromStart)
        (:Update
          ;;[1 1 1] If it has a location of 0,0,0 means this is exactly where it started
          (Transformation|SetRelativeLocation (Variables|Default|GetBumperMechanism) (Math|Vector|Lerp(Vector) "0, 0, 0" "0, 0,-70.000000" _bumpalpha) false false)
          ;;[1 1 1] Set the point light intensity to 0.0 to 5000 when hit. (The intsentity is set to 0.0 on the point light object viewport)
          (Rendering|Components|Light|SetIntensity (Variables|Default|GetPointLight) (Math|Float|Lerp 0.0 5e+03 _bumpalpha))
          ;;[1 1 1] Referse to a single number. This is our immisive boost. - EmmisiveBoost was taken from a material M_Bumper
          (Rendering|Material|SetScalarParameterValue (Variables|Default|GetBumperTopMID) "EmmisiveBoost" (Math|Float|Lerp 0.0 2e+01 _bumpalpha) :!class /Script/Engine.MaterialInstanceDynamic))))
    (:CastFailed
      (Timeline|BumpLerp PlayFromStart))))

(event EventBeginPlay)

(event Collision|EventActorBeginOverlap
  (params (OtherActor :type Actor%20Object%20Reference))
  ;[1 1 1] Checks if its a ball - Fire the pin, if it's not, dont
  (bind _asbp_ball (Utilities|Casting|CastToBp_Ball OtherActor))
  ;[1 1 1] If its a ball - Bump the ball (run the function called bump)
  (CallFunction|Bump _asbp_ball))

(event EventTick
  (params (DeltaSeconds :type Float%20%28single-precision%29)))

(fn ConstructionScript
  ;[1 1 1] Create a dynamic material to create a lighting affect on the material (Element index is applied to the mesh, the number of the element are different material channels)
  (bind _returnvalue (Rendering|Material|CreateDynamicMaterialInstance (Variables|Default|GetBumperMesh) 1 0 :!class /Script/Engine.PrimitiveComponent))
  ;[1 1 1] Store a reference to the material for later
  (Variables|Default|SetBumperTopMID _returnvalue))