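; Pinball ball actor that propels itself and sticks to the table surface beneath it.
; On BeginPlay it attaches a ball sound to the Ball component.
; Each Tick it adds a delta-time-scaled DefaultSpeed impulse as a velocity change, ignoring mass.
; It also traces down on Visibility and, for each hit, pushes the ball against the impact normal, scaled by TableStickyness and delta time.
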(event EventBeginPlay
  ;[1 1 1] Event BeginPlay
  (Audio|SpawnSoundAttached "/Game/Assets/Sounds/Pinball_BallLoose_Cue.Pinball_BallLoose_Cue" (Variables|Default|GetBall)))

(event Collision|EventActorBeginOverlap
  (params (OtherActor :type Actor%20Object%20Reference)))

(event EventTick
  (params (DeltaSeconds :type Float%20%28single-precision%29))
  (bind _returnvalue (Transformation|GetActorLocation))
  ;[1 1 1] Adding fake delta time / Vel change - Ignore any mass of the object make sure it get to the value it gets to big small move at that speed
  (Physics|AddImpulse (Variables|Default|GetBall) (* (Variables|Default|GetDefaultSpeed) DeltaSeconds) "None" true)
  ;[1 1 1] Look at the floor at all times /Stick to the ground
  (bind _outhits (Collision|MultiLineTraceByChannel _returnvalue (- _returnvalue "0, 0,500.000000") "TraceTypeQuery1" false 0 "None"))
  (bind _array_element (Utilities|Array|ForEachLoopwithBreak _outhits)
    (:LoopBody
      ;[1 1 1] Get the actor location
      (Physics|AddImpulse (Variables|Default|GetBall) (* (* (.ImpactNormal (Collision|BreakHitResult _array_element)) -1.0) (* (Variables|Default|GetTableStickyness) DeltaSeconds)) "None" true))))

(fn ConstructionScript)