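; Pinball flipper actor that serves as either a left or right flipper, chosen by the FlipType enum.
; The construction script picks the start and end rotations for that side, sets the resting pose and mirrors the right flipper with negative X scale.
; Flip and Flop events move the component between those rotations over FlipTime, with Flip also playing the flipper sound at world origin.
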(event Custom|Flip
  ;[1 1 1] When move is called it will gradually over a given time period go to the location and roation you have requested it to go to
  (Components|MoveComponentTo (Variables|Default|GetFlipper) "0, 0, 0" (Variables|Default|GetEndRotation) false false (Variables|Default|GetFlipTime) false)
  ;[1 1 1] Sound
  (Audio|PlaySoundatLocation "/Game/Assets/Sounds/Pinball_FlipperLeft_Cue.Pinball_FlipperLeft_Cue" "0, 0, 0"))

(event Custom|Flop
  ;[1 1 1] When move is called it will gradually over a given time period go to the location and roation you have requested it to go to
  (Components|MoveComponentTo (Variables|Default|GetFlipper) "0, 0, 0" (Variables|Default|GetStartRotation) false false (Variables|Default|GetFlipTime) false))

(event EventBeginPlay)

(event Collision|EventActorBeginOverlap
  (params (OtherActor :type Actor%20Object%20Reference)))

(event EventTick
  (params (DeltaSeconds :type Float%20%28single-precision%29)))

(fn ConstructionScript
  ;[1 1 1] What direction are they going to flip?
  (Variables|Default|SetStartRotation (Utilities|Select :Index (Variables|Default|GetFlipType) :NewEnumerator0 "0,20.000000,0" :NewEnumerator1 "0,-20.000000,0"))
  (Variables|Default|SetEndRotation (Utilities|Select :Index (Variables|Default|GetFlipType) :NewEnumerator0 "0,-20.000000,0" :NewEnumerator1 "0,20.000000,0"))
  ;[1 1 1] Starting rotation before hitting the flip button
  (Transformation|SetRelativeRotation (Variables|Default|GetFlipper) (Variables|Default|GetStartRotation) false false)
  ;[1 1 1] It asks if it the left or is it the right. If it is the right flip it. If it is the left keep it as it is.
  (switch Utilities|FlowControl|Switch|SwitchonFlipType (Variables|Default|GetFlipType)
    (:NewEnumerator1
      ;[1 1 1] This flips the flipper to make it the right flipper
      (Transformation|SetRelativeScale3D (Variables|Default|GetFlipper) "-1.000000,1.000000,1.000000"))))