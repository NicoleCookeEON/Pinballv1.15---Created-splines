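; A pinball drop target that sinks out of play with a bell sound when hit, labelled with a configurable letter.
; A hit moves the mesh down and disables its collision, then fires the OnDrop dispatcher.
; ResetTarget raises the mesh and restores collision, and BeginPlay binds an event to the pinball game mode's OnGameReset.
; The construction script writes DropLetter to the text render.
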(event Custom|Drop
  ;[1 1 1] Drop - When we want to drop it move -110 on z axis
  (Components|MoveComponentTo (Variables|Default|GetDTMesh) "0, 0,-110.000000" "0, 0, 0" false false 0.2 false)
  ;[1 1 1] Saftey procaution for no collision
  (Collision|SetCollisionEnabled (Variables|Default|GetDTMesh) "NoCollision")
  ;[1 1 1] When drops makes a sound
  (Audio|PlaySoundatLocation "/Game/Assets/Sounds/Pinball_Bell01_Cue.Pinball_Bell01_Cue" (Transformation|GetActorLocation)))

(event Custom|ResetTarget
  ;[1 1 1] ResetTarget - Set the move target back to default 0
  (Components|MoveComponentTo (Variables|Default|GetDTMesh) "0, 0,0.000000" "0, 0, 0" false false 0.2 false)
  ;[1 1 1] Saftey procaution for no collision
  (Collision|SetCollisionEnabled (Variables|Default|GetDTMesh) "QueryAndPhysics"))

(event EventBeginPlay
  ;[1 1 1] BeginPlay
  (bind _aspinball_game_mode (Utilities|Casting|CastToPinballGameMode (Game|GetGameMode)))
  (EventDispatchers|BindEventtoOnGameReset _aspinball_game_mode (EventDispatchers|CreateEvent :!event Custom|ResetTarget)))

(event Collision|EventActorBeginOverlap
  (params (OtherActor :type Actor%20Object%20Reference)))

(event EventTick
  (params (DeltaSeconds :type Float%20%28single-precision%29)))

(event Collision|EventHit
  (params (MyComp :type Primitive%20Component%20Object%20Reference) (Other :type Actor%20Object%20Reference) (OtherComp :type Primitive%20Component%20Object%20Reference) (bSelfMoved :type Boolean) (HitLocation :type Vector :default "0, 0, 0") (HitNormal :type Vector :default "0, 0, 0") (NormalImpulse :type Vector :default "0, 0, 0") (Hit :type Hit%20Result%20Structure%20%28by%20ref%29))
  ;[1 1 1] Event Hit - Always check on the stsatic mesh SimulationGenerationHitEvents is checked
  (CallFunction|Drop)
  ;[1 1 1] This is the Event Dispatcher
  (Default|CallOnDrop))

(fn ConstructionScript
  ;[1 1 1] This changes the text when changed in the default setting of DropLetter
  (Rendering|Components|TextRender|SetText (Variables|Default|GetTextRender) (Utilities|Text|ToText(String) (Variables|Default|GetDropLetter))))