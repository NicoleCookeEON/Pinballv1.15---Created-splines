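; BP_DrioTagetSet is a drop target set that builds a row of child actors from a string, one per character.
; Its Construction Script runs the parent's script, uppercases DropTargetString and splits it into characters.
; Each character adds a child actor component along relative X, stepped by the Post1-to-Post2 distance divided by character count plus one.
; The child actors are not yet given their letters, and the event graph is empty.
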(event EventBeginPlay)

(event Collision|EventActorBeginOverlap
  (params (OtherActor :type Actor%20Object%20Reference)))

(event EventTick
  (params (DeltaSeconds :type Float%20%28single-precision%29)))

(fn ConstructionScript
  ;[1 1 1] This node will do what its partent node would do in its own construction script. Has all its funcationality from its parent plus more
  (|CallParentFunction)
  (bind _output_get (Variables|Default|SetDropTargetString (Class|KismetStringLibrary|ToUpper (Variables|Default|GetDropTargetString))))
  ;[1 1 1] Its going to create a child actor every time it iterates through
  (for (_ _array_index) (Utilities|String|GetCharacterArrayfromString _output_get)
    ;[1 1 1] we are spawning a new actor thats parents to this as if it where a compentent of this actor
    (AddComponent|AddChildActorComponent false (Math|Transform|MakeTransform (Math|Vector|MakeVector (* _array_index (/ (Math|Vector|VectorLength (- (Variables|/Script/Engine.SceneComponent|GetRelativeLocation (Variables|Default|GetPost1)) (Variables|/Script/Engine.SceneComponent|GetRelativeLocation (Variables|Default|GetPost2)))) (Math|Conversions|ToFloat(Integer) (+ (Utilities|Array|Length (Utilities|String|GetCharacterArrayfromString _output_get)) 1)))) 0.0 0.0) "0, 0, 0" "1,1,1"))))