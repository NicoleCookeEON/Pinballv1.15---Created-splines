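; BP_Rail is a spline-based rail actor that builds a bent rail along a Spline component.
; The construction script adds a spline mesh component for each segment between neighbouring points, using the start mesh first, the end mesh last and the mid mesh between.
; Each piece takes its positions and tangents from the spline's two points in local space, so it follows the curve.
; The event graph has no active logic.
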(event EventBeginPlay)

(event Collision|EventActorBeginOverlap
  (params (OtherActor :type Actor%20Object%20Reference)))

(event EventTick
  (params (DeltaSeconds :type Float%20%28single-precision%29)))

(fn ConstructionScript
  (bind _spline (Variables|Default|GetSpline))
  (bind _spline_2 (Variables|Default|GetSpline))
  (bind _returnvalue (Spline|GetNumberOfSplinePoints _spline_2))
  (bind _returnvalue_2 (- _returnvalue 2))
  ;[1 1 1] This is going to bend the mesh that is set with this script
  ;[1 1 1] Look at the spline and count how many points are in it. Every point that is in there, add a mesh to the next point.
  (for _index (range 0 _returnvalue_2)
    ;[1 1 1] Sets the mesh (RailMid)
    (bind _returnvalue_3 (AddComponent|AddSplineMeshComponent false))
    ;[1 1 1] Check - See if the peice that is there (Current index) is also the index 0
    (if (== _index 0)
      ;[1 1 1] If true - This is the Rail Mouth Mesh
      (Components|StaticMesh|SetStaticMesh _returnvalue_3 (Variables|Default|GetRailStartMesh))
      (else
        ;[1 1 1] If true - This is the Rail End Mesh
        (if (== _index _returnvalue_2)
          (Components|StaticMesh|SetStaticMesh _returnvalue_3 (Variables|Default|GetRailEndMesh))
          (else
            ;[1 1 1] If False - This is the Rail End Mesh
            (Components|StaticMesh|SetStaticMesh _returnvalue_3 (Variables|Default|GetRailMidMesh))))))
    ;[1 1 1] Set these to corospond with the mesh just set
    (SplineMesh|SetStartandEnd _returnvalue_3 (.Location (Spline|GetLocationandTangentatSplinePoint _spline _index "Local")) (.Tangent (Spline|GetLocationandTangentatSplinePoint _spline _index "Local")) (.Location (Spline|GetLocationandTangentatSplinePoint _spline (+ _index 1) "Local")) (.Tangent (Spline|GetLocationandTangentatSplinePoint _spline (+ _index 1) "Local")) true :!class /Script/Engine.SplineMeshComponent)))