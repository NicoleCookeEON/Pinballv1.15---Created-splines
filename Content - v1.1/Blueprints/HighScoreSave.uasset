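; HighScoreSave holds an array of score entry structs for the game's high scores and finds the extremes among them.
; DetermineLowestScoreValue and DetermineHighestScoreValue each scan SaveStruct linearly, seeding from the first element and replacing it only on a strictly better match.
; Each returns both the matching struct and its array index, so ties resolve to the earliest entry.
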(fn DetermineLowestScoreValue
  ;[1 1 1] Check the score of each one of these stucts
  (for (_array_element _array_index) (Variables|Default|GetSaveStruct)
    ;[1 1 1] Is this the first element of the array
    (if (== _array_index 0)
      (LocalVariables|SetLowestScore (.score _array_element))
      (LocalVariables|SetLowestIndex _array_index)
      (else
        ;[1 1 1] Is the score currently greater than our known lowest score, if yes set, if not loop again
        (if (< (.score _array_element) (LocalVariables|GetLowestScore))
          (LocalVariables|SetLowestScore (.score _array_element))
          (LocalVariables|SetLowestIndex _array_index)))))
  ;[1 1 1] The struct itself is outputted
  (return (Utilities|Array|Get(acopy) (Variables|Default|GetSaveStruct) (LocalVariables|GetLowestIndex)) (LocalVariables|GetLowestIndex)))

(fn DetermineHighestScoreValue
  ;[1 1 1] Check the score of each one of these stucts
  (for (_array_element _array_index) (Variables|Default|GetSaveStruct)
    ;[1 1 1] Is this the first element of the array
    (if (== _array_index 0)
      (LocalVariables|SetHighestScore (.score _array_element))
      (LocalVariables|SetHighestIndex _array_index)
      (else
        ;[1 1 1] Is the score currently greater than our known lowest score, if yes set, if not loop again
        (if (> (.score _array_element) (LocalVariables|GetHighestScore))
          (LocalVariables|SetHighestScore (.score _array_element))
          (LocalVariables|SetHighestIndex _array_index)))))
  ;[1 1 1] The struct itself is outputted
  (return (Utilities|Array|Get(acopy) (Variables|Default|GetSaveStruct) (LocalVariables|GetHighestIndex)) (LocalVariables|GetHighestIndex)))