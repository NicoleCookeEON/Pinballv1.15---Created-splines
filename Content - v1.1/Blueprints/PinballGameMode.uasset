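; Pinball game mode that spawns balls and keeps the score.
; On BeginPlay it spawns a ball at the first found plunger's spawn location and binds to its destroyed event, which spawns a replacement every time.
; The BallsRemaining check is disconnected and EndGame is empty, so respawning never stops.
; AddScore multiplies incoming points by Multiplier, adds them to Score and returns the new total.
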(event Custom|SpawnBall
  ;[1 1 1] SpawnBall
  (bind _outactors (Actor|GetAllActorsOfClass "/Game/Blueprints/BP_Plunger.BP_Plunger_C"))
  (bind _returnvalue (Game|SpawnActorfromClass "/Game/Blueprints/Bp_Ball.Bp_Ball_C" (Math|Transform|MakeTransform (Default|GetBallSpawnLocation (Utilities|Array|Get(acopy) _outactors)) "0, 0, 0" "1,1,1") "Undefined" 0 0))
  ;[1 1 1] This is caused by an event dispatcher
  (Game|BindEventtoOnDestroyed _returnvalue (delegate Custom|OnBallDestroyed)))

(event Custom|EndGame
  ;[1 1 1] EndGame - How do you die?
)

(event Custom|OnBallDestroyed
  (params (DestroyedActor :type Actor%20Object%20Reference))
  ;[1 1 1] Get a message from the ball when it is destoryed
  (CallFunction|SpawnBall))

(event EventBeginPlay
  ;[1 1 1] BeginPlay
  (CallFunction|SpawnBall))

(event EventTick
  (params (DeltaSeconds :type Float%20%28single-precision%29)))

(fn ConstructionScript)

(fn AddScore
  (params (PointsToAdd :type Float%20%28single-precision%29))
  ;[1 1 1] Get the score, multiplying the current PointsToAdd, against a multiplyier value. Add that to the current score and set the current score to be that output
  ;;[1 1 1] Equal to score
  (bind _output_get (Variables|Default|SetScore (+ (* PointsToAdd (Variables|Default|GetMultiplier)) (Variables|Default|GetScore))))
  ;[1 1 1] Adding the current score, also can see what the current score has become
  (return _output_get))